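; Player controller for a third-person shooter that drives the possessed TPS character with camera-relative movement and look input.
; On possess it builds the equipped weapon's UI widget and binds to equip and unequip events, cleaning both up on unpossess.
; A camera-forward line trace lets Interact press BP_Button actors.
; A second camera trace, ignoring the character, supplies an aim override point at the impact.
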(event `self.ReceivePossess`
  (params (PossessedPawn :type "Pawn Object Reference"))
  (bind _astpscharacter_base (cast `/Game/Blueprint/Characters/Abstract/TPSCharacterBase` PossessedPawn))
  (bind _output_get (set `self.Controlled TPS Character` _astpscharacter_base))
  (`|ExecutionSequence`
    (:`then_0`
      (`self.Create Weapon UI` (`/Game/Blueprint/Characters/Abstract/TPSCharacterBase.Get Equipped Weapon` _output_get)))
    (:`then_1`
      (add `/Game/Blueprint/Characters/Abstract/TPSCharacterBase.On Equip` _output_get (`|CreateDelegate` :!event `Create Weapon UI`))
      (add `/Game/Blueprint/Characters/Abstract/TPSCharacterBase.On Unequip` _output_get (`|CreateDelegate` :!event `Clean Weapon UI`)))))

(event `self.ReceiveUnPossess`
  (params (UnpossessedPawn :type "Pawn Object Reference"))
  (`self.Clean Weapon UI`)
  (bind _controlled_tps_character (`self.Controlled TPS Character`)
    (:`then`
      (remove `/Game/Blueprint/Characters/Abstract/TPSCharacterBase.On Equip` _controlled_tps_character (`|CreateDelegate` :!event `Create Weapon UI`))
      (remove `/Game/Blueprint/Characters/Abstract/TPSCharacterBase.On Unequip` _controlled_tps_character (`|CreateDelegate` :!event `Clean Weapon UI`))
      (set `self.Controlled TPS Character` null))
    (:`else`)))

(event `InputAxis|TPS_MoveForward`
  (params (AxisValue :type "Float (single-precision)"))
  (bind _controlled_tps_character (`self.Controlled TPS Character`)
    (:`then`
      (`/Game/Blueprint/Characters/Abstract/TPSCharacterBase.Move` _controlled_tps_character (`KismetMathLibrary.GetForwardVector` (`PlayerCameraManager.GetCameraRotation` (`self.PlayerCameraManager`))) AxisValue))
    (:`else`)))

(event `InputAction|TPS_Interact`
  (params (Key :type "Key Structure"))
  (:`Pressed`
    (bind _hit_actor (`self.Cast Ray`))
    (bind _asbp_button (cast `/Game/Blueprint/Interactables/BP_Button` _hit_actor))
    (`/Game/Blueprint/Interactables/BP_Button.Interact` _asbp_button)))

(event `InputAxis|TPS_MoveRight`
  (params (AxisValue :type "Float (single-precision)"))
  (bind _controlled_tps_character (`self.Controlled TPS Character`)
    (:`then`
      (`/Game/Blueprint/Characters/Abstract/TPSCharacterBase.Move` _controlled_tps_character (`KismetMathLibrary.GetRightVector` (`PlayerCameraManager.GetCameraRotation` (`self.PlayerCameraManager`))) AxisValue))
    (:`else`)))

(event `InputAxis|TPS_Turn`
  (params (AxisValue :type "Float (single-precision)"))
  (`self.AddYawInput` AxisValue))

(event `InputAxis|TPS_LookUp`
  (params (AxisValue :type "Float (single-precision)"))
  (`self.AddPitchInput` AxisValue))

(fn `Cast Ray`
  (returns (`Hit Actor` :type "Actor Object Reference"))
  (bind _rootcomponent (`Actor.RootComponent` (`self.PlayerCameraManager`)))
  (bind _returnvalue (`SceneComponent.K2_GetComponentLocation` _rootcomponent))
  (bind _outhit (`KismetSystemLibrary.LineTraceSingle` _returnvalue (+ _returnvalue (* (`SceneComponent.GetForwardVector` _rootcomponent) (`self.Interaction Distance`))) "TraceTypeQuery1"))
  (return (`.HitActor` (`GameplayStatics.BreakHitResult` _outhit))))

(fn `Clean Weapon UI`
  (bind _weapon_ui_instance (`self.Weapon UI Instance`)
    (:`then`
      (`Widget.RemoveFromParent` _weapon_ui_instance)
      (set `self.Weapon UI Instance` null))
    (:`else`)))

(fn `Create Weapon UI`
  (params (`Equipped Weapon` :type "/Game/Blueprint/Weapons/Abstract/Weapon Object Reference"))
  (bind _weapon_ui_class (`/Game/Blueprint/Weapons/Abstract/Weapon.Weapon UI Class` `Equipped Weapon`))
  (`|ExecutionSequence`
    (:`then_0`
      (`self.Clean Weapon UI`))
    (:`then_1`
      (`/Engine/EditorBlueprintResources/StandardMacros.IsValid` `Equipped Weapon`
        (:`Is Valid`
          (if (`KismetSystemLibrary.IsValidClass` _weapon_ui_class)
            (bind _returnvalue (`|CreateWidget` _weapon_ui_class self))
            (bind _output_get (set `self.Weapon UI Instance` _returnvalue))
            (`UserWidget.AddToViewport` _output_get 0)))))))

(fn `Get Aim Override`
  (returns (`Does Override Aim?` :type Boolean) (`Target Point` :type "Vector Structure"))
  (bind _playercameramanager (`self.PlayerCameraManager`))
  (bind _returnvalue (`PlayerCameraManager.GetCameraLocation` _playercameramanager))
  (bind (_outhit _returnvalue_2) (`KismetSystemLibrary.LineTraceSingle` _returnvalue (+ _returnvalue (* (`KismetMathLibrary.GetForwardVector` (`PlayerCameraManager.GetCameraRotation` _playercameramanager)) (`self.Aim Range`))) "TraceTypeQuery3" false (`|MakeArray` (`self.Controlled TPS Character`) :!type "Actor Object Reference")))
  (return _returnvalue_2 (`.ImpactPoint` (`GameplayStatics.BreakHitResult` _outhit))))

(fn `UserConstructionScript`)