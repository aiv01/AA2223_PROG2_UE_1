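; Game-over GameMode that ranks the finished run and shows the leaderboard in GameOverUI with a mouse cursor.
; BeginPlay loads or creates the rank save (Slot 0) and appends the current run from Slot 1 to a working array.
; SortRank bubbles higher scores forward, shorter time winning ties, and drops the last entry.
; Slot 0 is re-saved without explicitly assigning the array back to the save object.
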(event `self.ReceiveBeginPlay`
  (bind _returnvalue (`GameplayStatics.LoadGameFromSlot` "Slot 0"))
  (bind _astpsrank_save (cast `/Game/Blueprint/UI/Save/TPSRankSave` _returnvalue)
    (:`then`
      (bind _output_get (set `self.As TPSRank Save` _astpsrank_save))
      (set `self.Total Player Rank` (`/Game/Blueprint/UI/Save/TPSRankSave.Total Rank` _output_get)))
    (:`CastFailed`
      (bind _returnvalue_2 (`GameplayStatics.CreateSaveGameObject` "/Game/Blueprint/UI/Save/TPSRankSave.TPSRankSave_C"))
      (bind _output_get_2 (set `self.As TPSRank Save` _returnvalue_2))
      (set `self.Total Player Rank` (`/Game/Blueprint/UI/Save/TPSRankSave.Total Rank` _output_get_2))))
  (bind _returnvalue_3 (`GameplayStatics.LoadGameFromSlot` "Slot 1"))
  (bind _astpsplayer_save (cast `/Game/Blueprint/UI/Save/TPSPlayerSave` _returnvalue_3))
  (`KismetArrayLibrary.Array_Add` (`self.Total Player Rank`) (`/Game/Blueprint/UI/Save/TPSPlayerSave.Curr Game Save` _astpsplayer_save))
  (bind (_rank _curr_score) (`self.Sort Rank`))
  (`GameplayStatics.SaveGameToSlot` (`self.As TPSRank Save`) "Slot 0")
  (bind _returnvalue_4 (`|CreateWidget` "/Game/Blueprint/UI/GameOverUI.GameOverUI_C"))
  (`UserWidget.AddToViewport` _returnvalue_4 0)
  (bind _output_get_3 (set `self.Curr UI` _returnvalue_4))
  (`/Game/Blueprint/UI/GameOverUI.Fill Rank` _output_get_3 _rank _curr_score)
  (set `PlayerController.bShowMouseCursor` true (`GameplayStatics.GetPlayerController` 0)))

(fn `Sort Rank`
  (returns (Rank :type "Array of /Game/Blueprint/UI/PlayerRankValue Structure") (`Curr Score` :type "/Game/Blueprint/UI/PlayerRankValue Structure"))
  (locals (`Curr Index` :type Integer) (`Last Index` :type Integer :default 0))
  (bind _total_player_rank (`self.Total Player Rank`))
  (bind _total_player_rank_2 (`self.Total Player Rank`))
  (bind (_output_name _output_score _output_time) (break `/Game/Blueprint/UI/PlayerRankValue` (`|GetArrayItem` _total_player_rank_2 (`local.Curr Index`))))
  (bind (_output_name_2 _output_score_2) (break `/Game/Blueprint/UI/PlayerRankValue` (`|GetArrayItem` _total_player_rank (`local.Last Index`))))
  (bind (_output_name_3 _output_score_3 _output_time_2) (break `/Game/Blueprint/UI/PlayerRankValue` (`|GetArrayItem` _total_player_rank_2 (`local.Last Index`))))
  (bind _output_get (set `local.Last Index` (- (`KismetArrayLibrary.Array_Length` (`self.Total Player Rank`)) 1)))
  (for _index (range (+ _output_get 1))
    (bind _output_get_2 (set `local.Curr Index` _index))
    (bind (_output_name_4 _output_score_4) (break `/Game/Blueprint/UI/PlayerRankValue` (`|GetArrayItem` _total_player_rank _output_get_2)))
    (if (<= _output_score_4 _output_score_2)
      (if (== _output_score_4 _output_score_2)
        (if (> _output_time _output_time_2)
          (`KismetArrayLibrary.Array_Swap` (`self.Total Player Rank`) (`local.Curr Index`) (`local.Last Index`) :!label _label))
        (else
          (goto _label)))))
  (`KismetArrayLibrary.Array_Remove` (`self.Total Player Rank`) (`local.Last Index`))
  (`GameplayStatics.SaveGameToSlot` (`self.As TPSRank Save`) "Slot 0")
  (return (`self.Total Player Rank`) (`/Game/Blueprint/UI/Save/TPSPlayerSave.Curr Game Save` (`self.As TPSPlayer Save`))))

(fn `UserConstructionScript`)