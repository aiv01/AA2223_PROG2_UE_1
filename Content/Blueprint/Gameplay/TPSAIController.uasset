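; AI controller for TPS characters that runs each pawn's own behavior tree and tracks the player by perception.
; On possess it caches the character and starts its Behavior tree; unpossessing clears the reference and stops the brain logic.
; Sight updates swap Blackboard keys between the visible player as Target and the last stimulus location when lost.
; Hearing filters for the player but takes no action, and StopAI is empty.
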(event `self.ReceivePossess`
  (params (PossessedPawn :type "Pawn Object Reference"))
  (bind _astpscharacter_base (cast `/Game/Blueprint/Characters/Abstract/TPSCharacterBase` PossessedPawn))
  (set `self.TPS_Character` _astpscharacter_base)
  (`|ExecutionSequence`
    (:`then_0`
      (`self.Run AI`))))

(event `self.ReceiveUnPossess`
  (params (UnpossessedPawn :type "Pawn Object Reference"))
  (set `self.TPS_Character` null)
  (`BrainComponent.StopLogic` (`self.BrainComponent`) ""))

(event `self.Sight.OnTargetPerceptionUpdated`
  (params (Actor :type "Actor Object Reference") (Stimulus :type "AIStimulus Structure"))
  (bind _blackboard (`self.Blackboard`))
  (bind _blackboard_2 (`self.Blackboard`))
  (if (== Actor (`GameplayStatics.GetPlayerPawn` 0))
    (if Stimulus_bSuccessfullySensed
      (`BlackboardComponent.SetValueAsObject` _blackboard "Target" Actor)
      (`BlackboardComponent.ClearValue` _blackboard_2 "Target Last Position Vector")
      (else
        (`BlackboardComponent.ClearValue` _blackboard "Target")
        (`BlackboardComponent.SetValueAsVector` _blackboard_2 "Target Last Position Vector" Stimulus_StimulusLocation)))))

(event `self.Hearing.OnTargetPerceptionUpdated`
  (params (Actor :type "Actor Object Reference") (Stimulus :type "AIStimulus Structure"))
  (if (== Actor (`GameplayStatics.GetPlayerPawn` 0))
    (if Stimulus_bSuccessfullySensed
      _)))

(fn `Run AI`
  (bind _tps_character (`self.TPS_Character`)
    (:`then`
      (bind _behavior (`/Game/Blueprint/Characters/Abstract/TPSCharacterBase.Behavior` _tps_character)
        (:`then`
          (`self.RunBehaviorTree` _behavior))
        (:`else`)))
    (:`else`)))

(fn `Stop AI`)

(fn `UserConstructionScript`)