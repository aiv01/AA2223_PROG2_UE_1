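; BP_InteractableDoor is a door actor meant to open and close by teleporting its Cube between relative origin and the OpenPosition component's location.
; The TPS_Jump press flips IsDoorOpen and calls OpenCloseDoor, which flips it back, so repeated presses take the same branch.
; EnableInput for player controller 0 is unconnected, and BeginPlay, overlap and Tick are empty.
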(event `self.ReceiveBeginPlay`)

(event `InputAction|TPS_Jump`
  (params (Key :type "Key Structure"))
  (:`Pressed`
    (set `self.Is Door Open` (not (`self.Is Door Open`)))
    (`self.Open/Close Door`)))

(fn `Open/Close Door`
  (if (`self.Is Door Open`)
    (`SceneComponent.K2_SetRelativeLocation` (`self.Cube`) (0.0 0.0 0.0) false true)
    (set `self.Is Door Open` false)
    (else
      (`SceneComponent.K2_SetRelativeLocation` (`self.Cube`) (`SceneComponent.RelativeLocation` (`self.Open Position`)) false true)
      (set `self.Is Door Open` true))))

(fn `UserConstructionScript`)