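; Enemy third-person shooter character Blueprint that manages a looping patrol route for its AI.
; On BeginPlay it writes the first PatrolPoints actor location to the "Curr Patrol" Blackboard key and resets the patrol index.
; IncrementPatrolPointIndex advances the index with modulo wraparound and writes the next point's location to the same key.
; Tick and overlap events are disabled.
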(event `self.ReceiveBeginPlay`
  (`parent.ReceiveBeginPlay`)
  (`BlackboardComponent.SetValueAsVector` (`AIBlueprintHelperLibrary.GetBlackboard` null) "Curr Patrol" (`self.K2_GetActorLocation` (`|GetArrayItem` (`self.Patrol Points`))))
  (set `self.Curr Patrol Point Index` 0))

(fn `Increment Patrol Point Index`
  (bind _output_get (set `self.Curr Patrol Point Index` (mod (+ (`self.Curr Patrol Point Index`) 1) (`KismetArrayLibrary.Array_Length` (`self.Patrol Points`)))))
  (`BlackboardComponent.SetValueAsVector` (`AIBlueprintHelperLibrary.GetBlackboard` null) "Curr Patrol" (`self.K2_GetActorLocation` (`|GetArrayItem` (`self.Patrol Points`) _output_get))))

(fn `UserConstructionScript`
  (`parent.UserConstructionScript`))