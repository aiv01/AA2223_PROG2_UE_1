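; BP_NextLevelMrg is a level-transition trigger that detects when two players are overlapping it.
; Begin overlap increments CollidingPlayers for TPSCharacterBase actors and prints "Next level reached!" when the count equals two.
; End overlap decrements the count for any actor, as its character cast is unwired.
; The OpenLevelByName call using NextLevelName is also disconnected, so no level loads.
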(event `self.ReceiveActorBeginOverlap`
  (params (OtherActor :type "Actor Object Reference"))
  (cast `/Game/Blueprint/Characters/Abstract/TPSCharacterBase` OtherActor)
  (set `self.Colliding Players` (+ (`self.Colliding Players`) 1))
  (if (== (`self.Colliding Players`) 2)
    (`KismetSystemLibrary.PrintString` "Next level reached!")))

(event `self.ReceiveActorEndOverlap`
  (params (OtherActor :type "Actor Object Reference"))
  (set `self.Colliding Players` (- (`self.Colliding Players`) 1)))

(fn `UserConstructionScript`)