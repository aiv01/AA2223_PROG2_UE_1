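; BP_Lives_Mgr is a manager Blueprint that tracks the player's remaining lives.
; TakeOneLife decrements LivesLeft, then reloads the current level or opens the game-over level at zero, and GetCurrentLivesCount exposes the count.
; The Construction Script zeroes LivesLeft and then sets it to LivesStartNumber, so each construction resets the count, with no persistence across level loads shown here.
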(fn `Get Current Lives Count`
  (returns (`Lives Left` :type Integer))
  (return (`self.Lives Left`)))

(fn `Take One Life`
  (set `self.Lives Left` (- (`self.Lives Left`) 1))
  (if (== (`self.Lives Left`) 0)
    (`GameplayStatics.OpenLevel` (`self.Game Over Scene Name`))
    (else
      (bind _returnvalue (`GameplayStatics.GetCurrentLevelName` true))
      (`GameplayStatics.OpenLevel` (`KismetStringLibrary.Conv_StringToName` _returnvalue)))))

(fn `UserConstructionScript`
  (set `self.Lives Left` 0)
  (if (== (`self.Lives Left`) 0)
    (set `self.Lives Left` (`self.Lives Start Number`))))