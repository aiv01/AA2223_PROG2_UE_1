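; Player manager that spawns two characters for the local player and lets them switch between the two with the TPS_Switch input.
; On BeginPlay it loads the save slot but spawns two TPSMannequins at numbered PlayerStarts, leaving the saved character lookups unwired.
; It possesses the first and binds both characters' death events.
; Switching re-possesses by the parity of a press counter.
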(event `self.ReceiveBeginPlay`
  (bind _astpsplayer_controller (cast `/Game/Blueprint/Gameplay/TPSPlayerController` (`GameplayStatics.GetPlayerController` 0)))
  (`self.EnableInput` _astpsplayer_controller)
  (bind _returnvalue (`GameplayStatics.LoadGameFromSlot` "Slot 1"))
  (bind _astpsplayer_save (cast `/Game/Blueprint/UI/Save/TPSPlayerSave` _returnvalue)
    (:`then`
      (`/Engine/EditorBlueprintResources/StandardMacros.IsValid` null
        (:`Is Valid`
          _)))
    (:`CastFailed`
      _))
  (`self.Assign Characters` "/Game/Blueprint/Characters/TPSMannequin.TPSMannequin_C" "/Game/Blueprint/Characters/TPSMannequin.TPSMannequin_C")
  (set `self.Switch Count` 1))

(event `InputAction|TPS_Switch`
  (params (Key :type "Key Structure"))
  (:`Pressed`
    (`self.Switch Character`)))

(fn `Assign Characters`
  (params (`Character 1` :type "/Game/Blueprint/Characters/Abstract/TPSCharacterBase Class Reference") (`Character 2` :type "/Game/Blueprint/Characters/Abstract/TPSCharacterBase Class Reference"))
  (bind _returnvalue (`|SpawnActorFromClass` `Character 1` (`self.Get Spawn Transform` 1) "AlwaysSpawn" "OverrideRootScale" null null))
  (set `self.Character 1` _returnvalue)
  (bind _returnvalue_2 (`|SpawnActorFromClass` `Character 2` (`self.Get Spawn Transform` 2) "AlwaysSpawn" "OverrideRootScale" null null))
  (set `self.Character 2` _returnvalue_2)
  ;[1 1 1] Assign the first character to the player controller
  (bind _astpsplayer_controller (cast `/Game/Blueprint/Gameplay/TPSPlayerController` (`GameplayStatics.GetPlayerController` 0)))
  (`Controller.UnPossess` _astpsplayer_controller)
  (`Controller.Possess` _astpsplayer_controller (`self.Character 1`))
  (add `/Game/Blueprint/Characters/Abstract/TPSCharacterBase.On Death` (`self.Character 1`) (`|CreateDelegate` (`self.Lives Mgr`) :!event `Take One Life`))
  (add `/Game/Blueprint/Characters/Abstract/TPSCharacterBase.On Death` (`self.Character 2`) (`|CreateDelegate` (`self.Lives Mgr`) :!event `Take One Life`)))

(fn `Get Spawn Transform`
  (params (`Player Position` :type Integer))
  (returns (ReturnValue :type "Transform Structure (by ref)"))
  (bind _astpsgame_mode_base (cast `/Game/Blueprint/Gameplay/TPSGameModeBase` (`GameplayStatics.GetGameMode`)))
  (return (`self.GetTransform` (`GameModeBase.K2_FindPlayerStart` _astpsgame_mode_base null (`KismetStringLibrary.Conv_IntToString` `Player Position`)))))

(fn `Switch Character`
  (bind _returnvalue (+ (`self.Switch Count`) 1))
  (set `self.Switch Count` _returnvalue)
  (bind _astpsplayer_controller (cast `/Game/Blueprint/Gameplay/TPSPlayerController` (`GameplayStatics.GetPlayerController` 0)))
  (`Controller.UnPossess` _astpsplayer_controller)
  (if (== (mod _returnvalue 2) 0)
    (`Controller.Possess` _astpsplayer_controller (`self.Character 1`))
    (else
      (`Controller.Possess` _astpsplayer_controller (`self.Character 2`)))))

(fn `UserConstructionScript`)